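; AI controller for the Flyeye enemy that steers it toward a target pawn.
; On possession it caches the pawn as a Flyeye, and a SetTargetPlayer event stores the target.
; Each tick, while both references are valid, it passes the look-at direction to the target into the Flyeye's MoveTowards at full scale, with no pathfinding or behavior tree in this graph.
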(event Custom|SetTargetPlayer
  (params (TargetPawn :type Pawn%20Object%20Reference))
  (Variables|Default|SetTargetPawn TargetPawn))

(event EventBeginPlay
  (|CallParentFunction) ; This node is disabled and will not be called.\nDrag off pins to build functionality.
)

(event EventTick
  (params (DeltaSeconds :type Float%20%28single-precision%29))
  (Utilities|IsValid (Variables|Default|GetOwningFlyeye)
    (:Is%20Valid
      (Utilities|IsValid (Variables|Default|GetTargetPawn)
        (:Is%20Valid
          (Default|MoveTowards (Variables|Default|GetOwningFlyeye) (Math|Vector|GetForwardVector (Math|Rotator|FindLookatRotation (Transformation|GetActorLocation (Variables|Default|GetOwningFlyeye)) (Transformation|GetActorLocation (Variables|Default|GetTargetPawn)))) 1.0))))))

(event EventPossess
  (params (PossessedPawn :type Pawn%20Object%20Reference))
  (bind _asbp_enemy_flyeye (Utilities|Casting|CastToBP_Enemy_FLYEYE PossessedPawn))
  (Variables|Default|SetOwningFlyeye _asbp_enemy_flyeye))

(fn ConstructionScript
  (|CallParentFunction))