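; Base action character Blueprint that handles incoming damage and a hit flash on its sprite.
; BeginPlay creates a dynamic material instance for the sprite.
; AnyDamage passes damage to the BPCHealthSystem component unless already defeated, then calls CallDefeated on defeat or TriggerFlash otherwise.
; TriggerFlash sets the material's flash color and multiplier, and the FadeSpriteFlash timeline fades the multiplier to zero at an adjustable play rate.
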(event Custom|TriggerFlash
  (params (FlashMultiplier :type Float%20%28single-precision%29) (FlashColor :type Linear%20Color%20Structure))
  ;[1 1 1] Damage Flash
  (Rendering|Material|SetScalarParameterValue (Variables|Default|GetDynamicSpriteMat) "FlashMultiplier" FlashMultiplier :!class /Script/Engine.MaterialInstanceDynamic)
  (Rendering|Material|SetVectorParameterValue (Variables|Default|GetDynamicSpriteMat) "FlashColor" FlashColor :!class /Script/Engine.MaterialInstanceDynamic)
  (Components|Timeline|SetPlayRate (Variables|Default|GetFadeSpriteFlash) (Variables|Default|GetSpriteFlashPlayRate))
  (bind _alpha (Timeline|FadeSpriteFlash PlayFromStart)
    (:Update
      (Rendering|Material|SetScalarParameterValue (Variables|Default|GetDynamicSpriteMat) "FlashMultiplier" (Math|Float|Lerp FlashMultiplier 0.0 _alpha) :!class /Script/Engine.MaterialInstanceDynamic))))

(event EventBeginPlay
  (bind _returnvalue (Rendering|Material|CreateDynamicMaterialInstance (Variables|Default|GetSprite) 0 0 "None" :!class /Script/Engine.PrimitiveComponent))
  (Variables|Default|SetDynamicSpriteMat _returnvalue))

(event Collision|EventActorBeginOverlap
  (params (OtherActor :type Actor%20Object%20Reference)))

(event EventTick
  (params (DeltaSeconds :type Float%20%28single-precision%29)))

(event Game|Damage|EventAnyDamage
  (params (Damage :type Float%20%28single-precision%29) (DamageType :type Damage%20Type%20Object%20Reference) (InstigatedBy :type Controller%20Object%20Reference) (DamageCauser :type Actor%20Object%20Reference))
  ;[1 1 1] Apply Damage and destroy actor after health is below 0
  (if (not (Variables|/Game/Blueprints/Components/BPC_HealthSystem.BPC_HealthSystem_C|GetIsDefeated (Variables|Default|GetBPC_HealthSystem)))
    (Default|ReceiveDamage (Variables|Default|GetBPC_HealthSystem) Damage)
    (if (Variables|/Game/Blueprints/Components/BPC_HealthSystem.BPC_HealthSystem_C|GetIsDefeated (Variables|Default|GetBPC_HealthSystem))
      (Default|CallDefeated)
      (else
        (CallFunction|TriggerFlash 5.0 "(R=1.000000,G=0.618204,B=0.066385,A=1.000000)")))))

(fn ConstructionScript)