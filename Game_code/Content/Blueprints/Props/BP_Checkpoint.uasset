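; Checkpoint prop that registers itself as the active checkpoint in the GM_Action game mode when the player reaches it.
; On BeginPlay it caches the game mode, then its Trigger overlap filters for BP_Player.
; A DoOnce limits activation to the first player touch, which also swaps the Cube's material as a visual marker, so revisiting an older checkpoint does not make it active again.
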(event OnComponentBeginOverlap(Trigger)
  (params (OverlappedComponent :type Primitive%20Component%20Object%20Reference) (OtherActor :type Actor%20Object%20Reference) (OtherComp :type Primitive%20Component%20Object%20Reference) (OtherBodyIndex :type Integer) (bFromSweep :type Boolean) (SweepResult :type Hit%20Result%20Structure%20%28by%20ref%29))
  (Utilities|Casting|CastToBP_Player OtherActor)
  (Utilities|FlowControl|DoOnce false
    (:Completed
      (Variables|/Game/Blueprints/GM_Action.GM_Action_C|SetActiveCheckpoint (Variables|Default|GetGMAction) self)
      (Rendering|Material|SetMaterial (Variables|Default|GetCube) 0 "/Engine/EngineDebugMaterials/VertexColorViewMode_BlueOnly.VertexColorViewMode_BlueOnly"))))

(event EventBeginPlay
  (bind _asgm_action (Utilities|Casting|CastToGM_Action (Game|GetGameMode)))
  (Variables|Default|SetGMAction _asgm_action))

(event Collision|EventActorBeginOverlap
  (params (OtherActor :type Actor%20Object%20Reference)))

(event EventTick
  (params (DeltaSeconds :type Float%20%28single-precision%29)))

(fn ConstructionScript)